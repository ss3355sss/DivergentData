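; BP_DvBlockOut_Box is a level blockout box that labels its height in meters on its front and back.
; The construction script derives local dimensions from BoxSize, then sets two text components to the Z-scaled height and places each just outside opposite X faces, centered in Y and Z.
; Reset restores BoxSize to a one-meter cube and reruns construction.
; The event graph holds only disabled default events.
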(fn `Reset`
  (set `self.BoxSize` (100.0 100.0 100.0))
  (`self.RerunConstructionScript`))

(fn `UserConstructionScript`
  (locals (Local_Width :type "Float (double-precision)") (Local_Height :type "Float (double-precision)") (Local_Depth :type "Float (double-precision)") (Local_Offset :type "Float (double-precision)" :default 0.1))
  (bind (_returnvalue_x _returnvalue_y _returnvalue_z) (`KismetMathLibrary.BreakVector` (`self.GetActorScale3D`)))
  (bind _heighttextrendercomponent_front (`self.HeightTextRenderComponent_Front`))
  (bind _heighttextrendercomponent_back (`self.HeightTextRenderComponent_Back`))
  (bind (_boxsize_x _boxsize_y _boxsize_z) (`KismetMathLibrary.BreakVector` (`self.BoxSize`)))
  (bind _result (`|FormatText` "{length} m" (/ (* (`local.Local_Height`) _returnvalue_z) 100.0)))
  (`parent.UserConstructionScript`)
  (`|ExecutionSequence`
    (:`then_0`
      (set `local.Local_Width` _boxsize_x)
      (set `local.Local_Height` _boxsize_z)
      (set `local.Local_Depth` _boxsize_y))
    (:`then_1`
      (`TextRenderComponent.K2_SetText` _heighttextrendercomponent_front _result)
      (`SceneComponent.K2_SetRelativeLocation` _heighttextrendercomponent_front (`KismetMathLibrary.MakeVector` (+ (`local.Local_Width`) (`local.Local_Offset`)) (/ (`local.Local_Depth`) 2.0) (/ (`local.Local_Height`) 2.0)) false false))
    (:`then_2`
      (`TextRenderComponent.K2_SetText` _heighttextrendercomponent_back _result)
      (`SceneComponent.K2_SetRelativeLocation` _heighttextrendercomponent_back (`KismetMathLibrary.MakeVector` (* (`local.Local_Offset`) -1.0) (/ (`local.Local_Depth`) 2.0) (/ (`local.Local_Height`) 2.0)) false false))))